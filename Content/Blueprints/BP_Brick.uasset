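; BP_Brick is a destructible brick that loses one point of BrickStrength each time a BP_Ball hits it.
; At zero strength it spawns a scaled-up explosion emitter at its location and destroys itself.
; UpdateBrickColor maps strengths one to three to different cube materials.
; It is called only from the Construction Script, so the hit event leaves the color unchanged.
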(event `self.ReceiveHit`
  (params (MyComp :type "PrimitiveComponent Object Reference") (Other :type "Actor Object Reference") (OtherComp :type "PrimitiveComponent Object Reference") (bSelfMoved :type Boolean) (HitLocation :type "Vector Structure") (HitNormal :type "Vector Structure") (NormalImpulse :type "Vector Structure") (Hit :type "HitResult Structure (by ref)"))
  (cast `/Game/Blueprints/BP_Ball` Other)
  (bind _result (`/Engine/EditorBlueprintResources/StandardMacros.DecrementInt` (`self.BrickStrength`))
    (:`  `
      (if (== _result 0)
        (`GameplayStatics.SpawnEmitterAtLocation` "/Game/StarterContent/Particles/P_Explosion.P_Explosion" (`self.K2_GetActorLocation`) (struct) (3.0 3.0 3.0))
        (`self.K2_DestroyActor`)))))

(fn `UpdateBrickColor`
  (bind _cube (`self.Cube`))
  (switch `int` (`self.BrickStrength`)
    (:`1`
      (`PrimitiveComponent.SetMaterial` _cube 0 "/Game/Materials/MI_Yellow.MI_Yellow"))
    (:`2`
      (`PrimitiveComponent.SetMaterial` _cube 0 "/Game/Materials/MI_Red.MI_Red"))
    (:`3`
      (`PrimitiveComponent.SetMaterial` _cube 0 "/Game/Materials/MI_Green.MI_Green"))))

(fn `UserConstructionScript`
  (`self.UpdateBrickColor`))