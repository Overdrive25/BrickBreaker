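; BP_Ball is the physics ball of a paddle-and-brick game, launched along X with a velocity-change impulse when play begins.
; On every hit it raises BallSpeed by a fixed step and clamps its velocity to exactly that magnitude, so it keeps its direction while speeding up.
; Hits on actors tagged "brick" update the score through the HUD of the player's BP_Paddle pawn, cached at start.
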(event `self.ReceiveBeginPlay`
  (`PrimitiveComponent.AddImpulse` (`self.Sphere`) (1200.0 0.0 0.0) "None" true)
  (bind _asbp_paddle (cast `/Game/Blueprints/BP_Paddle` (`GameplayStatics.GetPlayerPawn` 0)))
  (set `self.As BP Paddle` _asbp_paddle))

(event `self.ReceiveHit`
  (params (MyComp :type "PrimitiveComponent Object Reference") (Other :type "Actor Object Reference") (OtherComp :type "PrimitiveComponent Object Reference") (bSelfMoved :type Boolean) (HitLocation :type "Vector Structure") (HitNormal :type "Vector Structure") (NormalImpulse :type "Vector Structure") (Hit :type "HitResult Structure (by ref)"))
  (bind _sphere (`self.Sphere`))
  (bind _ballspeed (`self.BallSpeed`))
  (set `self.BallSpeed` (+ (`self.BallSpeed`) 10.0))
  (bind _returnvalue (`PrimitiveComponent.GetPhysicsLinearVelocity` _sphere "None"))
  (`PrimitiveComponent.SetPhysicsLinearVelocity` _sphere (`KismetMathLibrary.ClampVectorSize` _returnvalue _ballspeed _ballspeed) false "None")
  (if (`self.ActorHasTag` Other "brick")
    (`/Game/Widgets/WBP_PlayerHUD.Update Score` (`/Game/Blueprints/BP_Paddle.PlayerHUD` (`self.As BP Paddle`)))))

(fn `UserConstructionScript`)